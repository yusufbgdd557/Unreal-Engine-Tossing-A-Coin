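; Player Blueprint for a touch-controlled coin toss that detects which side of the coin rests on the table.
; A touch launches the coin upward with a random spin, then locks further touches for about a second.
; Tick checks the upper and lower collision components for table overlap, rechecking after a short delay to confirm rest.
; A DoOnce per side then re-enables touch and prints that side as a debug string.
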(event `InputTouch`
  (params (Location :type "Vector Structure") (FingerIndex :type "ETouchIndex Enum"))
  (:`Pressed`
    (if (`self.CanTouch`)
      (`PrimitiveComponent.AddImpulse` (`self.Coin`) (0.0 0.0 750.0) "None" true)
      (`KismetSystemLibrary.Delay` 0.02)
      (`PrimitiveComponent.AddAngularImpulseInDegrees` (`self.Coin`) (`KismetMathLibrary.MakeVector` (`KismetMathLibrary.RandomFloatInRange` 700.0 2000.0)) "None" true)
      (set `self.CanTouch` false)
      (`KismetSystemLibrary.Delay` 1.0)
      (set `self.CanTouch` true))))

(event `self.ReceiveTick`
  (params (DeltaSeconds :type "Float (single-precision)"))
  (`|ExecutionSequence`
    (:`then_0`
      (if (`PrimitiveComponent.IsOverlappingComponent` (`self.Lower_Collision`) (`self.Table`))
        (`KismetSystemLibrary.Delay` 0.5)
        (if (`PrimitiveComponent.IsOverlappingComponent` (`self.Lower_Collision`) (`self.Table`))
          (`/Engine/EditorBlueprintResources/StandardMacros.DoOnce` false :!label _label
            (:`Completed`
              (set `self.CanTouch` true)
              (`KismetSystemLibrary.PrintString` "Lower")))
          (else
            (goto _label :!via `Reset`)))))
    (:`then_1`
      (if (`PrimitiveComponent.IsOverlappingComponent` (`self.Upper_Collision`) (`self.Table`))
        (`KismetSystemLibrary.Delay` 0.5)
        (if (`PrimitiveComponent.IsOverlappingComponent` (`self.Upper_Collision`) (`self.Table`))
          (`/Engine/EditorBlueprintResources/StandardMacros.DoOnce` false :!label _label_2
            (:`Completed`
              (set `self.CanTouch` true)
              (`KismetSystemLibrary.PrintString` "Upper")))
          (else
            (goto _label_2 :!via `Reset`)))))))

(fn `UserConstructionScript`)